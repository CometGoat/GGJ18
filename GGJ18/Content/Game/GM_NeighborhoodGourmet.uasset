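; Game mode for Neighborhood Gourmet that runs the endless tile road and the viewer score.
; Zip spawns four tiles past the last one, takes its food chance, randomizes HUD chill level, and uses a timeline to drive speed and lerp.
; CalculateMultiplier converts recent food-talk flags into a viewer multiplier and speech border color.
; Tick grows or shrinks the clamped viewer count from that multiplier, bonus and HUD talk delay.
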(event `self.ReceiveBeginPlay`
  (bind _outactors (`GameplayStatics.GetAllActorsOfClass` "/Game/Blueprints/BP_Tile.BP_Tile_C"))
  (for _array_element _outactors
    (if (`/Game/Blueprints/BP_Tile.LastTile` _array_element)
      (set `self.LastTile` _array_element)))
  (set `self.W_HUD` (`/Game/Blueprints/BP_Van.W_HUD` (cast `/Game/Blueprints/BP_Van` (`Controller.K2_GetPawn` (`GameplayStatics.GetPlayerController` 0)) :!pure true))))

(event `self.ReceiveTick`
  (params (DeltaSeconds :type "Float (single-precision)"))
  (`self.CalculateViewers`))

(event `Zip`
  (for _index (range 4)
    (bind _returnvalue (`|SpawnActorFromClass` "/Game/Blueprints/BP_Tile.BP_Tile_C" (`KismetMathLibrary.MakeTransform` (+ (`self.K2_GetActorLocation` (`self.LastTile`)) (* (1200.0 0.0 0.0) (+ _index 1)))) "AlwaysSpawn" "OverrideRootScale" null null))
    (set `/Game/Blueprints/BP_Tile.Zipping` true _returnvalue)
    (`/Game/Blueprints/BP_Tile.Zip` _returnvalue)
    (if (== _index 3)
      (bind _output_get (set `self.LastTile` _returnvalue))
      (set `self.FoodChance` (`/Game/Blueprints/BP_Tile.FoodChance` _output_get))
      (set `/Game/UI/Widgets/W_SpeechBox.ChillLevel` (`KismetMathLibrary.RandomIntegerInRange` 1 6) (`self.W_HUD`))))
  (bind (_direction _speed _poslerpalpha) (`Timeline|ZipValue` :!via `PlayFromStart`)
    (:`Update`
      (set `self.Speed` _speed)
      (bind _output_get_2 (set `self.SpeedLerp` _poslerpalpha)))
    (:`Finished`
      (bind _outactors (`GameplayStatics.GetAllActorsOfClass` "/Game/Blueprints/BP_Tile.BP_Tile_C"))
      (for _array_element _outactors
        (set `/Game/Blueprints/BP_Tile.Zipping` false _array_element)))))

(event `CalculateMultiplier`
  (set `self.FoodCount` 0)
  (for _array_element (`self.TalkinBoutFood`)
    (if _array_element
      (`/Engine/EditorBlueprintResources/StandardMacros.IncrementInt` (`self.FoodCount`))))
  (bind _output_get (set `self.ViewerMultiplier` (select `int` (`self.FoodCount`) :`0` -1.0 :`1` -0.5 :`2` 0.1 :`3` 1.0 :`4` 2.0 :`5` 3.0 :!type "Float (single-precision)")))
  (`Border.SetBrushColor` (`/Game/UI/Widgets/W_SpeechBox.SpeechBorder` (`self.W_HUD`)) (select `int` (`self.FoodCount`) :`0` (struct :`R` 1.0 :`G` 0.124772 :`B` 0.124772 :`A` 1.0) :`1` (struct :`R` 1.0 :`G` 0.5 :`B` 0.5 :`A` 1.0) :`2` (struct :`R` 1.0 :`G` 0.459 :`B` 0.164 :`A` 1.0) :`3` (struct :`R` 1.0 :`G` 0.752942 :`B` 0.226966 :`A` 1.0) :`4` (struct :`R` 0.5 :`G` 1.0 :`B` 0.5 :`A` 1.0) :`5` (struct :`R` 0.125 :`G` 1.0 :`B` 0.125 :`A` 1.0) :!type "LinearColor Structure")))

(event `CalculateViewers`
  (set `self.Viewers` (`KismetMathLibrary.Clamp` (+ (`KismetMathLibrary.FTrunc` (* (`self.ViewerBonus`) (* (* (`self.ViewerMultiplier`) (- 8.0 (* (`/Game/UI/Widgets/W_SpeechBox.TalkDelayMax` (`self.W_HUD`)) 7.0))) (* (`GameplayStatics.GetWorldDeltaSeconds`) 8.0)))) (`self.Viewers`)) 1 100000000)))

(fn `UserConstructionScript`)