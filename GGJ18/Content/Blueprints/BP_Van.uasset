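; BP_Van is a van actor with an orthographic camera and a click-to-rev mechanic that triggers a "zip" move.
; Left clicks add to Rev, which decays each tick and tilts the Sphere component in proportion.
; Pushing Rev past its threshold resets it, calls Zip on every BP_Tile, and plays the ZipAnim timeline to rotate and lift the Sphere, pausing decay until it finishes.
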(event `self.ReceiveTick`
  (params (DeltaSeconds :type "Float (single-precision)"))
  (`self.ReduceRev`))

(event `Key|LeftMouseButton`
  (params (Key :type "Key Structure"))
  (:`Pressed`
    (bind _output_get (set `self.Rev` (+ (`self.Rev`) (`self.RevBoostRate`))))
    (if (> _output_get 8.0)
      (`self.Zip`)
      (else
        (`KismetSystemLibrary.PrintString` (`KismetStringLibrary.Conv_DoubleToString` _output_get))))))

(event `Zip`
  (bind _sphere (`self.Sphere`))
  (`KismetSystemLibrary.PrintString` "Zip!")
  (set `self.Zipping` true)
  (set `self.Rev` 0.0)
  (bind _outactors (`GameplayStatics.GetAllActorsOfClass` "/Game/Blueprints/BP_Tile.BP_Tile_C"))
  (for _array_element _outactors
    (`/Game/Blueprints/BP_Tile.Zip` _array_element))
  (bind (_direction _rotation _height) (`Timeline|ZipAnim` :!via `PlayFromStart`)
    (:`Update`
      (`SceneComponent.K2_SetRelativeRotation` _sphere (`KismetMathLibrary.MakeRotator` 0.0 _rotation) false false)
      (`SceneComponent.K2_SetRelativeLocation` _sphere (`KismetMathLibrary.MakeVector` -100.0 0.0 _height) false false))
    (:`Finished`
      (set `self.Zipping` false))))

(event `ReduceRev`
  (if (not (`self.Zipping`))
    (bind _output_get (set `self.Rev` (`KismetMathLibrary.FClamp` (- (`self.Rev`) (* (`GameplayStatics.GetWorldDeltaSeconds`) (`self.RevReductionRate`))) 0.0 8.0)))
    (`SceneComponent.K2_SetRelativeRotation` (`self.Sphere`) (`KismetMathLibrary.MakeRotator` 0.0 (* (/ (`self.RevAngle`) 8.0) _output_get)) false false)))

(fn `UserConstructionScript`
  (`CameraComponent.SetOrthoWidth` (`self.Camera`) (`self.CameraDistance`)))