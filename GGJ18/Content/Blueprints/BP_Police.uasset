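; BP_Police is the police actor that drives in to arrest the player's van as soon as it spawns.
; On BeginPlay it jumps to a fixed start point, then the ArrestPlayer timeline drives its world X position with Y and Z held at zero.
; It plays a tire screech after a short delay and flags the controlled BP_Van as Caught without waiting for the drive to finish.
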(event `self.ReceiveBeginPlay`
  (`self.K2_SetActorLocation` (3600.0 0.0 0.0))
  (`self.DriveToPlayer`)
  (set `/Game/Blueprints/BP_Van.Caught` true (cast `/Game/Blueprints/BP_Van` (`Controller.K2_GetPawn` (`GameplayStatics.GetPlayerController` 0)) :!pure true)))

(event `DriveToPlayer`
  (`self.ScreechTires`)
  (bind (_direction _location) (`Timeline|ArrestPlayer` :!via `PlayFromStart`)
    (:`Update`
      (`self.K2_SetActorLocation` (`KismetMathLibrary.MakeVector` _location)))))

(event `ScreechTires`
  (`KismetSystemLibrary.Delay` 0.5)
  (`GameplayStatics.PlaySound2D` "/Game/Sound/VanScreech/CUE_VanScreech.CUE_VanScreech"))

(fn `UserConstructionScript`)