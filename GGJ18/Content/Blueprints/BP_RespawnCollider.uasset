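; BP_RespawnCollider is a trigger actor that extends a chain of BP_Tile actors along X.
; When a tile begins overlapping its Box, it spawns a new tile at a fixed X offset from LastTile, makes that the new LastTile and calls Zip on it.
; The previous LastTile is stored in TileToFree, but the delayed destroy logic is disconnected, so this Blueprint never removes old tiles.
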(event `self.Box.OnComponentBeginOverlap`
  (params (OverlappedComponent :type "PrimitiveComponent Object Reference") (OtherActor :type "Actor Object Reference") (OtherComp :type "PrimitiveComponent Object Reference") (OtherBodyIndex :type Integer) (bFromSweep :type Boolean) (SweepResult :type "HitResult Structure (by ref)"))
  (bind _lasttile (`self.LastTile`))
  (cast `/Game/Blueprints/BP_Tile` OtherActor)
  (set `self.TileToFree` _lasttile)
  (bind _returnvalue (`|SpawnActorFromClass` "/Game/Blueprints/BP_Tile.BP_Tile_C" (`KismetMathLibrary.MakeTransform` (+ (`self.K2_GetActorLocation` _lasttile) (1200.0 0.0 0.0))) "AlwaysSpawn" "OverrideRootScale" null null))
  (bind _output_get (set `self.LastTile` _returnvalue))
  (`/Game/Blueprints/BP_Tile.Zip` _output_get))

(fn `UserConstructionScript`)