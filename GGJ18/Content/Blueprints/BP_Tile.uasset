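; Tile actor for the Neighborhood Gourmet game mode that slides along negative X during a zip move.
; While Zipping is true, Zip lerps it from a saved start toward a fixed offset using the game mode's SpeedLerp, re-calling itself after a one-frame-length Delay instead of using Tick.
; When Zipping ends, a DoOnce resets so the next zip re-captures its start.
; Construction averages two random rolls into a center-weighted FoodChance.
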(event `self.ReceiveBeginPlay`
  (set `self.StartZipVector` (`self.K2_GetActorLocation`)))

(event `Zip`
  (bind _startzipvector (`self.StartZipVector`))
  (`|ExecutionSequence`
    (:`then_0`
      (`/Engine/EditorBlueprintResources/StandardMacros.DoOnce` true :!label _label
        (:`Completed`
          (set `self.StartZipVector` (`self.K2_GetActorLocation`)))))
    (:`then_1`
      (if (`self.Zipping`)
        (`self.K2_SetActorLocation` (`KismetMathLibrary.VLerp` _startzipvector (- _startzipvector (3600.0 0.0 0.0)) (`/Game/Game/GM_NeighborhoodGourmet.SpeedLerp` (cast `/Game/Game/GM_NeighborhoodGourmet` (`GameplayStatics.GetGameMode`) :!pure true))))
        (`KismetSystemLibrary.Delay` (`GameplayStatics.GetWorldDeltaSeconds`))
        (`self.Zip`)
        (else
          (goto _label :!via `Reset`))))))

(fn `UserConstructionScript`
  (set `self.FoodChance` (/ (+ (`KismetMathLibrary.RandomFloatInRange` 20.0 100.0) (`KismetMathLibrary.RandomFloatInRange` 20.0 100.0)) 2.0)))